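; BP_Data is a Blueprint that reads a trivia question from a data table and prints it, apparently as a test of the lookup.
; On BeginPlay it looks up the row named by QuestionRow in the TriviaQuestions table.
; When the row is found, it takes the Category, Question and Answer fields and shows each with Print String.
; A missing row is not handled, and the construction script is empty.
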(event EventBeginPlay
  (bind _returnvalue (Utilities|GetDataTableRow "/Game/TestQuestions/Data/TriviaQuestions.TriviaQuestions" (Variables|Default|GetQuestionRow))
    (:then
      (Variables|Default|SetCategory (.Category (Utilities|Struct|BreakStructure_DataTable _returnvalue)))
      (Variables|Default|SetQuestion (.Question (Utilities|Struct|BreakStructure_DataTable _returnvalue)))
      (Variables|Default|SetAnswer (.Answer (Utilities|Struct|BreakStructure_DataTable _returnvalue)))
      (Development|PrintString (Variables|Default|GetCategory) true true "(R=0.000000,G=0.660000,B=1.000000,A=1.000000)" 1e+01)
      (Development|PrintString (Variables|Default|GetQuestion) true true "(R=0.000000,G=0.660000,B=1.000000,A=1.000000)" 1e+01)
      (Development|PrintString (Variables|Default|GetAnswer) true true "(R=0.000000,G=0.660000,B=1.000000,A=1.000000)" 1e+01))))

(fn ConstructionScript)